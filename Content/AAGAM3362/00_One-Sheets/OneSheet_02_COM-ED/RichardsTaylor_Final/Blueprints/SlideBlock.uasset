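; SlideBlock is a Blueprint with a Cube that slides vertically up or down from a shared rest height.
; SlideUp and SlideDown play separate timelines that lerp the Cube's relative location toward a raised or lowered offset.
; ResetUp and ResetDown reverse the matching timeline to bring it back.
; Nothing in its own graphs triggers these four events.
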(event `SlideUp`
  (bind (_direction _uslide) (`Timeline|UpSlide` :!label _label)
    (:`Update`
      (`SceneComponent.K2_SetRelativeLocation` (`self.Cube`) (`KismetMathLibrary.VLerp` (0.0 0.0 50.0) (0.0 0.0 160.0) _uslide) false false))))

(event `ResetUp`
  (goto _label :!via `Reverse`))

(event `SlideDown`
  (bind (_direction _dslide) (`Timeline|DownSlide` :!label _label_2)
    (:`Update`
      (`SceneComponent.K2_SetRelativeLocation` (`self.Cube`) (`KismetMathLibrary.VLerp` (0.0 0.0 50.0) (0.0 0.0 -40.0) _dslide) false false))))

(event `ResetDown`
  (goto _label_2 :!via `Reverse`))

(fn `UserConstructionScript`)