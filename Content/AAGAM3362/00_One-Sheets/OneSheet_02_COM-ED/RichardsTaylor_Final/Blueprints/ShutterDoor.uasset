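; Six-panel shutter door that opens when a puzzle is solved and closes again when a ball is destroyed.
; PuzzleSolved, guarded by IsDoorOpen, plays the OpenDoor timeline, which lerps each panel's relative location from its stored start point to its end point.
; BallDestroyed clears the flag and reverses the same timeline to slide the panels back.
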(event `Puzzle Solved`
  (if (not (`self.IsDoorOpen`))
    (set `self.IsDoorOpen` true)
    (bind (_direction _animation) (`Timeline|Open Door` :!label _label)
      (:`Update`
        (`SceneComponent.K2_SetRelativeLocation` (`self.Bottom`) (`KismetMathLibrary.VLerp` (`self.BottomStartingPoint`) (`self.BottomEndingPoint`) _animation) false false)
        (`SceneComponent.K2_SetRelativeLocation` (`self.BottomLeft`) (`KismetMathLibrary.VLerp` (`self.BottomLeftStartingPoint`) (`self.BottomLeftEndingPoint`) _animation) false false)
        (`SceneComponent.K2_SetRelativeLocation` (`self.BottomRight`) (`KismetMathLibrary.VLerp` (`self.BottomRightStartingPoint`) (`self.BottomRightEndingPoint`) _animation) false false)
        (`SceneComponent.K2_SetRelativeLocation` (`self.Top`) (`KismetMathLibrary.VLerp` (`self.TopStartingPoint`) (`self.TopEndingPoint`) _animation) false false)
        (`SceneComponent.K2_SetRelativeLocation` (`self.TopLeft`) (`KismetMathLibrary.VLerp` (`self.TopLeftStartingPoint`) (`self.TopLeftEndingPoint`) _animation) false false)
        (`SceneComponent.K2_SetRelativeLocation` (`self.TopRight`) (`KismetMathLibrary.VLerp` (`self.TopRightStartingPoint`) (`self.TopRightEndingPoint`) _animation) false false)))))

(event `Ball Destroyed`
  (set `self.IsDoorOpen` false)
  (goto _label :!via `Reverse`))

(fn `UserConstructionScript`)