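; TiltBlock is a block actor whose Cube tilts 20 degrees to either side and back.
; TiltRight and TiltLeft each play their own timeline, which lerps the Cube's relative rotation from level toward that side's angle.
; ResetRight and ResetLeft reverse the matching timeline to undo the tilt.
; Nothing in the Blueprint calls these events, and its Tick and overlap handlers are empty.
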(event `TiltRight`
  (bind (_direction _rtilt) (`Timeline|RightTilt` :!label _label)
    (:`Update`
      (`SceneComponent.K2_SetRelativeRotation` (`self.Cube`) (`KismetMathLibrary.RLerp` (struct) (struct :`Roll` 20.0) _rtilt) false false))))

(event `ResetRight`
  (goto _label :!via `Reverse`))

(event `TiltLeft`
  (bind (_direction _ltilt) (`Timeline|LeftTilt` :!label _label_2)
    (:`Update`
      (`SceneComponent.K2_SetRelativeRotation` (`self.Cube`) (`KismetMathLibrary.RLerp` (struct) (struct :`Roll` -20.0) _ltilt true) false false))))

(event `ResetLeft`
  (goto _label_2 :!via `Reverse`))

(fn `UserConstructionScript`)