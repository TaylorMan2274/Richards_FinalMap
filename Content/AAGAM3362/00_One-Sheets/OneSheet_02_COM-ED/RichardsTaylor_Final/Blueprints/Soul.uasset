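; Soul is a collectible pickup that counts toward winning the level.
; When an actor with "Character" in its name overlaps the Touch component, it increments SoulNum on the player's FirstPersonCharacter_h once and prints the count.
; Reaching four souls opens WinScreen.
; The first soul also raises the Wall actor and lowers it after a delay before destroying itself, while other non-winning pickups are destroyed immediately.
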(event `self.Touch.OnComponentBeginOverlap`
  (params (OverlappedComponent :type "PrimitiveComponent Object Reference") (OtherActor :type "Actor Object Reference") (OtherComp :type "PrimitiveComponent Object Reference") (OtherBodyIndex :type Integer) (bFromSweep :type Boolean) (SweepResult :type "HitResult Structure (by ref)"))
  (`/Engine/EditorBlueprintResources/StandardMacros.DoOnce` false
    (:`Completed`
      (if (`KismetStringLibrary.Contains` (`KismetSystemLibrary.GetObjectName` OtherActor) "Character")
        (`/Engine/EditorBlueprintResources/StandardMacros.DoOnce` false
          (:`Completed`
            (bind _result (`/Engine/EditorBlueprintResources/StandardMacros.IncrementInt` (`/Game/FirstPersonBP/Blueprints/FirstPersonCharacter_h.SoulNum` (cast `/Game/FirstPersonBP/Blueprints/FirstPersonCharacter_h` (`GameplayStatics.GetPlayerCharacter` 0) :!pure true)))
              (:`  `
                (`KismetSystemLibrary.PrintString` (`KismetStringLibrary.Conv_IntToString` _result))
                (if (>= _result 4)
                  (`GameplayStatics.OpenLevel` "WinScreen")
                  (elif (== _result 1)
                    (bind _returnvalue (`GameplayStatics.GetActorOfClass` "/Game/AAGAM3362/00_One-Sheets/OneSheet_02_COM-ED/RichardsTaylor_Final/Blueprints/Wall.Wall_C"))
                    (`/Game/AAGAM3362/00_One-Sheets/OneSheet_02_COM-ED/RichardsTaylor_Final/Blueprints/Wall.RaiseWall` _returnvalue)
                    (`KismetSystemLibrary.Delay` 10.0)
                    (bind _returnvalue_2 (`GameplayStatics.GetActorOfClass` "/Game/AAGAM3362/00_One-Sheets/OneSheet_02_COM-ED/RichardsTaylor_Final/Blueprints/Wall.Wall_C"))
                    (`/Game/AAGAM3362/00_One-Sheets/OneSheet_02_COM-ED/RichardsTaylor_Final/Blueprints/Wall.LowerWall` _returnvalue_2)
                    (`self.K2_DestroyActor`)
                    (else
                      (`self.K2_DestroyActor`))))))))))))

(fn `UserConstructionScript`)